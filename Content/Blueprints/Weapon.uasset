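; Automatic hitscan weapon Blueprint that fires repeatedly until StopFireWeapon is called.
; FireWeapon runs on a looping timer, line-tracing forward from LaserBeam with debug drawing, damaging EnemyCharacter hits and spawning enemy or default impact effects.
; A DoOnce starts attached looping gunfire audio and muzzle flash once per burst.
; StopFireWeapon resets it, clears the timer and destroys stored effect and sound components; the cooldown logic is left disconnected.
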(event Custom|FireWeapon
  (bind _laserbeam (Variables|Default|GetLaserBeam))
  (bind _laserspawn (Variables|Default|GetLaserSpawn))
  (bind _returnvalue (Transformation|GetWorldLocation _laserbeam))
  (Utilities|FlowControl|Sequence
    (:then_0
      (bind _returnvalue_2 (Utilities|Time|SetTimerbyFunctionName 0 "FireWeapon" 0.05 true)))
    (:then_1
      ;[1 1 1] Sound & Muzzle Flash FX
      (Utilities|FlowControl|DoOnce false
        (:Completed
          (Utilities|FlowControl|Sequence
            (:then_0
              (bind _returnvalue_3 (Audio|SpawnSoundAttached "/Game/Audio/AssaultRifle_ShotLoop01_Stereo.AssaultRifle_ShotLoop01_Stereo" _laserspawn "None" "0, 0, 0" "0, 0, 0" "KeepRelativeOffset" true 2.0 1.0 0.0 0 0 false)))
            (:then_1
              (bind _returnvalue_4 (Effects|SpawnEmitterAttached "/Game/GunFX/ParticleSystems/Weapons/AssaultRifle/Muzzle/P_AssaultRifle_MF.P_AssaultRifle_MF" _laserspawn "None" (Transformation|GetWorldLocation _laserspawn) (Transformation|GetWorldRotation _laserspawn) "1.000000,1.000000,1.000000" "KeepWorldPosition")))))))
    (:then_2
      ;[1 1 1] Bullets (RayCasting)
      (bind _outhit (Collision|LineTraceByChannel _returnvalue (+ _returnvalue (* (Math|Vector|GetForwardVector (Transformation|GetWorldRotation _laserbeam)) (Math|Conversions|ToVector(Float) (Variables|Default|GetWeapon%20Range)))) "TraceTypeQuery1" false 0 "ForOneFrame"))
      (bind _output_get (Variables|Default|SetHit%20Actor (.HitActor (Collision|BreakHitResult _outhit))))
      (bind _asenemy_character (Utilities|Casting|CastToEnemyCharacter _output_get)
        (:then
          (bind _returnvalue_5 (Effects|SpawnEmitteratLocation "/Game/FX/EnemyImpact.EnemyImpact" (.ImpactPoint (Collision|BreakHitResult _outhit)) (Math|Conversions|RotationFromXVector (.ImpactNormal (Collision|BreakHitResult _outhit)))))
          (Utilities|FlowControl|Sequence
            (:then_0
              (Utilities|FlowControl|Delay 0.2)
              (Components|DestroyComponent _returnvalue_5))
            (:then_1
              (Default|ReceiveDamage _asenemy_character (Variables|Default|GetWeaponDamage)))))
        (:CastFailed
          (bind _returnvalue_6 (Effects|SpawnEmitteratLocation "/Game/GunFX/ParticleSystems/Weapons/AssaultRifle/Impacts/P_AssaultRifle_IH.P_AssaultRifle_IH" (.ImpactPoint (Collision|BreakHitResult _outhit)) (Math|Conversions|RotationFromXVector (.ImpactNormal (Collision|BreakHitResult _outhit))))))))))

(event Custom|StopFireWeapon
  (bind _laserspawn (Variables|Default|GetLaserSpawn))
  (Utilities|FlowControl|Sequence
    (:then_0
      ;[1 1 1] Sound & Muzzle Flash FX
      (Utilities|FlowControl|DoOnce false) ; enters at Reset
    )
    (:then_1
      (Components|DestroyComponent (stale Custom|FireWeapon _returnvalue_4))
      (Components|DestroyComponent (stale Custom|FireWeapon _returnvalue_6)))
    (:then_2
      (Utilities|Time|ClearandInvalidateTimerbyHandle (stale Custom|FireWeapon _returnvalue_2)))
    (:then_3
      (Components|DestroyComponent (stale Custom|FireWeapon _returnvalue_3)))))

(fn ConstructionScript)